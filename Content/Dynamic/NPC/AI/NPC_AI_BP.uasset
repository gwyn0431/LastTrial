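; AI controller for the patrolling guard NPC, running its behavior tree and feeding it perception results.
; On begin play it sets up the patrol blackboard and starts the guard behavior tree.
; Perception updates set or clear the blackboard enemy key for actors without the "Enemy" tag, based on whether they are sensed.
; Each tick, it sets the guard's aiming flag for animation whenever a focus actor is valid.
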(event OnTargetPerceptionUpdated(AIPerception)
  (params (Actor :type Actor%20Object%20Reference) (Stimulus :type AI%20Stimulus%20Structure))
  (bind _blackboardcomp (Variables|Default|GetBlackBoardComp))
  (bind _enemykey (Variables|Default|GetEnemyKey))
  ;[1 1 1] Setting Enemy Key if Sensed someone
  (if (not (Actor|ActorHasTag Actor "Enemy"))
    (if (.bSuccessfullySensed (Utilities|Struct|BreakAIStimulus Stimulus))
      (AI|Components|Blackboard|SetValueasObject _blackboardcomp _enemykey Actor)
      (else
        (AI|Components|Blackboard|ClearValue _blackboardcomp _enemykey)))))

(event EventBeginPlay
  ;[1 1 1] Initialise using BB & BT (+ set BBComp var)
  (bind _blackboardcomponent (Class|AIController|UseBlackboard "/Game/Dynamic/NPC/AI/PatrolData.PatrolData"))
  (AI|RunBehaviorTree "/Game/Dynamic/NPC/AI/GuardBehaviour.GuardBehaviour")
  (Variables|Default|SetBlackBoardComp _blackboardcomponent))

(event EventTick
  (params (DeltaSeconds :type Float%20%28single-precision%29))
  ;[1 1 1] Setting IsAiming bool var for proper animation
  (bind _asbp_patrolling_guard (Utilities|Casting|CastToBP_PatrollingGuard (Pawn|GetControlledPawn)))
  (Variables|/Game/Dynamic/NPC/Behaviour/BP_PatrollingGuard.BP_PatrollingGuard_C|SetIsAiming _asbp_patrolling_guard (Utilities|IsValid (Class|AIController|GetFocusActor))))

(fn ConstructionScript)